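; Player controller for GetTheGun that swaps a default pawn for either a VR pawn or a first-person character.
; On possessing a DefaultPawn, it destroys that pawn and checks whether a head-mounted display is enabled.
; It then spawns BP_VRPawn or BP_FirstPersonCharacter at the first PlayerStart found and possesses it, so the possess event itself handles platform selection.
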(event `self.ReceivePossess`
  (params (PossessedPawn :type "Pawn Object Reference"))
  (bind _asdefault_pawn (cast `DefaultPawn` PossessedPawn))
  (`/Engine/EditorBlueprintResources/StandardMacros.IsValid` _asdefault_pawn
    (:`Is Valid`
      (`self.K2_DestroyActor` PossessedPawn)
      (bind _outactors (`GameplayStatics.GetAllActorsOfClass` "/Script/Engine.PlayerStart"))
      (if (`HeadMountedDisplayFunctionLibrary.IsHeadMountedDisplayEnabled`)
        (bind _returnvalue (`self.GetTransform` (`|GetArrayItem` _outactors)))
        (bind _returnvalue_2 (`|SpawnActorFromClass` "/Game/Core/Characters/Player/BP_VRPawn.BP_VRPawn_C" _returnvalue "Undefined" "MultiplyWithRoot" null null))
        (`self.Possess` _returnvalue_2)
        (else
          (bind _returnvalue_3 (`|SpawnActorFromClass` "/Game/Core/Characters/Player/BP_FirstPersonCharacter.BP_FirstPersonCharacter_C" _returnvalue "Undefined" "MultiplyWithRoot" null null))
          (`self.Possess` _returnvalue_3))))))

(fn `UserConstructionScript`)